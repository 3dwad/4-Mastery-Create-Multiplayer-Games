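; Multiplayer player character that fires a weapon and shows debug feedback for damage and death.
; The local player gets a crosshair widget, and left click calls the weapon's server fire.
; Body material changes and a right-click test string pass through server-to-multicast event pairs, while HealthComponent events trigger client-named draw events.
; SpawnSomething places a testing actor ahead along control yaw; unconnected nodes hold older weapon-attach and debug logic.
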(event OnHealthZero(HealthComponent)
  (CallFunction|DrawDeathClient))

(event OnTakeDamage(HealthComponent)
  (params (Damage :type Float%20%28single-precision%29) (CurrentHealth :type Float%20%28single-precision%29))
  (CallFunction|DrawDamageClient))

(event Custom|SetBodyMaterial_Server
  (params (MaterialIndex :type Integer))
  (CallFunction|SetBodyMaterialMulticast MaterialIndex))

(event Custom|SetBodyMaterial_Multicast
  (params (MaterialIndex :type Integer))
  (Rendering|Material|SetMaterial (Variables|Character|GetMesh) 0 (Utilities|Array|Get(acopy) (Variables|Default|GetBodyMaterials) MaterialIndex)))

(event Custom|SpawnSomething
  (Game|SpawnActorfromClass "/Game/Blueprints/BP_TestingActor.BP_TestingActor_C" (Math|Transform|MakeTransform (+ (Transformation|GetActorLocation) (* (Math|Vector|GetForwardVector (Math|Rotator|MakeRotator 0.0 0.0 (.yaw (Pawn|GetControlRotation :!class /Script/Engine.Pawn)))) 1.5e+02)) "0, 0, 0" "1,1,1") "Undefined" 0 0))

(event Custom|PrintOnServer
  (CallFunction|PrintMulticast (+ (Transformation|GetActorLocation) "0, 0,100.000000")))

(event Custom|Print_Multicast
  (params (NewParam :type Vector))
  (Rendering|Debug|DrawDebugString NewParam "TestString" 0 "(R=0.000000,G=0.090555,B=1.000000,A=1.000000)" 5.0))

(event Custom|DrawDamage_Client
  (Rendering|Debug|DrawDebugString (+ (Transformation|GetActorLocation) "0, 0,70.000000") "Damage!!!" 0 "(R=1.000000,G=0.337081,B=0.000000,A=1.000000)" 5.0))

(event Custom|DrawDeath_Client
  (Rendering|Debug|DrawDebugString (+ (Transformation|GetActorLocation) "0, 0,70.000000") "Death!!!" 0 "(R=1.000000,G=0.337081,B=0.000000,A=1.000000)" 5.0))

(event EventBeginPlay
  (if (Pawn|IsLocallyControlled)
    (bind _returnvalue (UserInterface|CreateWidget "/Game/UI/WBP_Cross.WBP_Cross_C"))
    (UserInterface|Viewport|AddtoViewport _returnvalue 0)))

(event EventTick
  (params (DeltaSeconds :type Float%20%28single-precision%29)))

(event EventOnFire)

(event Input|MouseEvents|LeftMouseButton
  (params (Key :type Key%20Structure :default "None"))
  (:Pressed
    (Class|CGWeapon|FireServer (Variables|Default|GetWeapon))))

(event Input|MouseEvents|RightMouseButton
  (params (Key :type Key%20Structure :default "None"))
  (:Pressed
    (CallFunction|PrintonServer)))

(fn ConstructionScript)